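; BP_Pickup_Base is the base class for pickups, tracking an active state and the visibility of its PickupSprite.
; It activates on BeginPlay, setting IsActive and showing the sprite.
; Deactivate hides and disables pickups flagged StartedInLevel so Activate can restore them, and destroys all others.
; ShouldBePickedUp always returns true here, and the file contains no overlap or collection logic.
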(event `self.ReceiveBeginPlay`
  (`self.Activate`))

(event `Deactivate`
  (if (`self.StartedInLevel`)
    (set `self.IsActive` false)
    (`SceneComponent.SetVisibility` (`self.PickupSprite`) false false)
    (else
      (`self.K2_DestroyActor`))))

(event `Activate`
  (set `self.IsActive` true)
  (`SceneComponent.SetVisibility` (`self.PickupSprite`) true false))

(fn `ShouldBePickedUp`
  (returns (ShouldBePickedUp :type Boolean))
  (return true))

(fn `UserConstructionScript`)