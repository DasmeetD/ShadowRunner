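; Base pickup Blueprint that shows a floating LetterE indicator while the 2DSideScrollerCharacter overlaps it.
; Begin overlap unhides LetterE and restarts a timeline whose Oscillation track lerps it between the relative locations of the Start and End components.
; End overlap hides LetterE and stops the timeline.
; It contains no input or collection logic.
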(event `self.ReceiveActorBeginOverlap`
  (params (OtherActor :type "Actor Object Reference"))
  (cast `/Game/2DSideScrollerBP/Blueprints/2DSideScrollerCharacter` OtherActor)
  (`SceneComponent.SetHiddenInGame` (`self.LetterE`) false false)
  (bind (_direction _oscillation) (`Timeline|Timeline_0` :!via `PlayFromStart` :!label _label)
    (:`Update`
      (`SceneComponent.K2_SetRelativeLocation` (`self.LetterE`) (`KismetMathLibrary.VLerp` (`SceneComponent.RelativeLocation` (`self.Start`)) (`SceneComponent.RelativeLocation` (`self.End`)) _oscillation) false false))))

(event `self.ReceiveActorEndOverlap`
  (params (OtherActor :type "Actor Object Reference"))
  (cast `/Game/2DSideScrollerBP/Blueprints/2DSideScrollerCharacter` OtherActor)
  (`SceneComponent.SetHiddenInGame` (`self.LetterE`) true false)
  (goto _label :!via `Stop`))

(fn `UserConstructionScript`)