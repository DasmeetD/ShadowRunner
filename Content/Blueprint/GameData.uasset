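; GameData is a game-instance-style Blueprint that tracks level progression and checkpoint respawning.
; It loads, restarts or advances through LevelList by index, with NextLevel resetting checkpoint progress.
; Checkpoint actors are mapped by number on Init and immediately after restart or advance calls to open a level.
; OnCheckpointHit keeps the highest number reached, which RestartLevel uses to set the respawn location and PlayerRespawned flag.
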(event `self.ReceiveInit`
  (`self.GetCheckpointsInLevel`))

(fn `GetCheckpointsInLevel`
  (`BlueprintMapLibrary.Map_Clear` (`self.Checkpoints`))
  (bind _outactors (`GameplayStatics.GetAllActorsOfClass` "/Game/Blueprint/Checkpoints/Checkpoint.Checkpoint_C"))
  (for _array_element _outactors
    (`BlueprintMapLibrary.Map_Add` (`self.Checkpoints`) (`/Game/Blueprint/Checkpoints/Checkpoint.CheckpointNumber` _array_element) _array_element)))

(fn `LoadLevel`
  (params (LevelNumber :type Integer))
  (bind _levellist (`self.LevelList`))
  (if (>= LevelNumber (`KismetArrayLibrary.Array_Length` _levellist))
    (`KismetSystemLibrary.PrintString` "Trying to access non existant level" true true (struct :`R` 1.0 :`A` 1.0))
    (else
      (set `self.CurrentLevel` LevelNumber)
      (`GameplayStatics.OpenLevel` (`|GetArrayItem` _levellist LevelNumber)))))

(fn `NextLevel`
  (bind _result (`/Engine/EditorBlueprintResources/StandardMacros.IncrementInt` (`self.CurrentLevel`))
    (:`  `
      (if (>= _result (`KismetArrayLibrary.Array_Length` (`self.LevelList`)))
        (`KismetSystemLibrary.PrintString` "Trying to access non existant level" true true (struct :`R` 1.0 :`A` 1.0))
        (else
          (`GameplayStatics.OpenLevel` (`|GetArrayItem` (`self.LevelList`) _result))
          (`self.GetCheckpointsInLevel`)
          (set `self.bHasHitCheckpoint` false)
          (set `self.CurrentCheckPoint` 0)
          (set `self.bPlayerRespawned` true))))))

(fn `OnCheckpointHit`
  (params (CheckpointNumber :type Integer))
  (set `self.bHasHitCheckpoint` true)
  (if (> CheckpointNumber (`self.CurrentCheckPoint`))
    (set `self.CurrentCheckPoint` CheckpointNumber)))

(fn `RestartLevel`
  (bind (_value _returnvalue) (`BlueprintMapLibrary.Map_Find` (`self.Checkpoints`) (`self.CurrentCheckPoint`)))
  (`GameplayStatics.OpenLevel` (`|GetArrayItem` (`self.LevelList`) (`self.CurrentLevel`)))
  (`self.GetCheckpointsInLevel`)
  (if (and (`self.bHasHitCheckpoint`) (> (`BlueprintMapLibrary.Map_Length` (`self.Checkpoints`)) 0))
    (if _returnvalue
      (set `self.PlayerRespawnLocation` (`Actor.K2_GetActorLocation` _value))
      (set `self.bPlayerRespawned` true))))