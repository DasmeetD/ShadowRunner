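; PickupManager tracks the pickups placed in the level and can activate them all at once.
; On BeginPlay it gathers every BP_Pickup_Base and BP_Commandable_Pickup_Base actor into separate arrays, flagging each as StartedInLevel.
; The ActivateAllPickups event loops through both arrays and calls Activate on each entry.
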(event `ActivateAllPickups`
  (for _array_element (`self.Pickups`)
    (`/Game/Pickups/BaseClass/BP_Pickup_Base.Activate` _array_element))
  (for _array_element_2 (`self.CommandablePickups`)
    (`/Game/Pickups/BaseClass/BP_Commandable_Pickup_Base.Activate` _array_element_2)))

(event `self.ReceiveBeginPlay`
  (`KismetArrayLibrary.Array_Clear` (`self.Pickups`))
  (`KismetArrayLibrary.Array_Clear` (`self.CommandablePickups`))
  (bind _outactors (`GameplayStatics.GetAllActorsOfClass` "/Game/Pickups/BaseClass/BP_Pickup_Base.BP_Pickup_Base_C"))
  (for _array_element _outactors
    (set `/Game/Pickups/BaseClass/BP_Pickup_Base.StartedInLevel` true _array_element)
    (`KismetArrayLibrary.Array_Add` (`self.Pickups`) _array_element))
  (bind _outactors_2 (`GameplayStatics.GetAllActorsOfClass` "/Game/Pickups/BaseClass/BP_Commandable_Pickup_Base.BP_Commandable_Pickup_Base_C"))
  (for _array_element_2 _outactors_2
    (set `/Game/Pickups/BaseClass/BP_Commandable_Pickup_Base.StartedInLevel` true _array_element_2)
    (`KismetArrayLibrary.Array_Add` (`self.CommandablePickups`) _array_element_2)))

(fn `UserConstructionScript`)