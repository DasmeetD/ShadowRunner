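; Checkpoint actor for a 2D side scroller that records the player's progress when first touched.
; The fire effect starts hidden at BeginPlay.
; When the side-scroller character first overlaps the capsule, it latches a hit flag and passes its checkpoint number to the GameData game instance.
; It then reveals the fire and plays the torch sound.
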(event `self.ReceiveBeginPlay`
  (`SceneComponent.SetVisibility` (`self.Fire`) false false))

(event `self.Capsule.OnComponentBeginOverlap`
  (params (OverlappedComponent :type "PrimitiveComponent Object Reference") (OtherActor :type "Actor Object Reference") (OtherComp :type "PrimitiveComponent Object Reference") (OtherBodyIndex :type Integer) (bFromSweep :type Boolean) (SweepResult :type "HitResult Structure (by ref)"))
  (if (not (`self.bPlayerHasHIt`))
    (cast `/Game/2DSideScrollerBP/Blueprints/2DSideScrollerCharacter` OtherActor)
    (set `self.bPlayerHasHIt` true)
    (bind _asgame_data (cast `/Game/Blueprint/GameData` (`GameplayStatics.GetGameInstance`)))
    (`/Game/Blueprint/GameData.OnCheckpointHit` _asgame_data (`self.CheckpointNumber`))
    (`SceneComponent.SetVisibility` (`self.Fire`) true false)
    (`AudioComponent.Play` (`self.Torch_Cue`) 0.0)))

(fn `UserConstructionScript`)